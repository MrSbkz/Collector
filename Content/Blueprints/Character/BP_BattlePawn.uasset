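; BP_BattlePawn is the battle pawn, whose camera toggles between its own view and an overview of the battle table.
; On BeginPlay it caches the first BP_BattleTable's camera transform and its own camera's starting world transform.
; SwitchCamera uses a FlipFlop to play or reverse a timeline that lerps the single camera component between those transforms.
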(event `self.ReceiveBeginPlay`
  (bind _outactors (`GameplayStatics.GetAllActorsOfClass` "/Game/Blueprints/Actor/Table/BP_BattleTable.BP_BattleTable_C"))
  (if (> (`KismetArrayLibrary.Array_Length` _outactors) 0)
    (bind _cameratransform (`/Game/Blueprints/Actor/Table/BP_BattleTable.GetCameraTransform` (`|GetArrayItem` _outactors)))
    (set `self.TableCameraTransform` _cameratransform)
    (set `self.CameraTransform` (`SceneComponent.K2_GetComponentToWorld` (`self.Camera`)))))

(event `PlayerInterface.SwitchCamera`
  (`/Engine/EditorBlueprintResources/StandardMacros.FlipFlop`
    (:`A`
      (bind (_direction _cameratrack) (`Timeline|SwitchCameraTimeline` :!label _label)
        (:`Update`
          (`SceneComponent.K2_SetWorldTransform` (`self.Camera`) (`KismetMathLibrary.TLerp` (`self.CameraTransform`) (`self.TableCameraTransform`) _cameratrack) false false))))
    (:`B`
      (goto _label :!via `Reverse`))))

(fn `UserConstructionScript`)