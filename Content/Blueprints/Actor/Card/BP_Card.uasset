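; BP_Card is a card actor that shows its data on a WBP_Card widget component and animates picking from the hand.
; Picking hides the other hand cards through the owner's DeckComponent and moves the card from its highlight spot to an owner-supplied location.
; Cancelling shows them again, returns the card to its initial location, then notifies a callback object.
; All movement, including a general move-to-location event, uses timeline-driven lerps.
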(event `self.SetCardUI`
  (params (CardData :type "CardDetails Structure (by ref)"))
  (bind _widgetcomponent (`self.WidgetComponent`)
    (:`then`
      (bind _aswbp_card (cast `/Game/Blueprints/UI/Widgets/Card/WBP_Card` (`WidgetComponent.GetWidget` _widgetcomponent)))
      (`/Game/Blueprints/UI/Widgets/Card/WBP_Card.UpdateCardDetails` _aswbp_card CardData))
    (:`else`)))

(event `InteractionInterface.Pick`
  (set `self.IsPicked` true)
  (`DeckComponent.HideOrShowHandCards` (`self.GetComponentByClass` (`self.GetOwner`) "/Script/Collector.DeckComponent") self true)
  (bind _returnvalue (message `PlayerInterface.GetPickedCardLocation` (`self.GetOwner`)))
  (bind (_direction _movecardtrack) (`Timeline|PickCardTimeline` :!via `PlayFromStart`)
    (:`Update`
      (`self.K2_SetActorLocation` (`KismetMathLibrary.VLerp` (`self.HighlightLocation`) _returnvalue _movecardtrack)))))

(event `InteractionInterface.CancelPicking`
  (params (CallbackObject :type "AwaitableObject Object Reference"))
  (set `self.IsPicked` false)
  (`DeckComponent.HideOrShowHandCards` (`self.GetComponentByClass` (`self.GetOwner`) "/Script/Collector.DeckComponent") self false)
  (bind (_direction _movecardtrack) (`Timeline|CancelPickingTimeline` :!via `PlayFromStart`)
    (:`Update`
      (`self.K2_SetActorLocation` (`KismetMathLibrary.VLerp` (`self.K2_GetActorLocation`) (`self.InitialLocation`) _movecardtrack)))
    (:`Finished`
      (`AwaitableObject.OnFinished` CallbackObject))))

(event `self.MoveToLocation`
  (params (Location :type "Vector Structure (by ref)"))
  (bind (_direction _movementtrack) (`Timeline|MoveToLocationTimeline` :!via `PlayFromStart`)
    (:`Update`
      (`self.K2_SetActorLocation` (`KismetMathLibrary.VLerp` (`self.K2_GetActorLocation`) Location _movementtrack)))))

(fn `UserConstructionScript`)